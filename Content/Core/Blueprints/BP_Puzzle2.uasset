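; BP_Puzzle2 is an interactable puzzle actor that opens the W_Puzzle2 widget for the first player.
; Interact creates and stores the widget, adds it to the viewport, switches input to Game and UI, and disables character movement, with no restore in this graph.
; Start and Finish only call the parent implementations.
; The spline is only read for debug prints at BeginPlay, and the construction script adds another debug print.
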(event `self.ReceiveBeginPlay`
  (bind _spline (`self.Spline`))
  (bind (_returnvalue_inputkey _returnvalue_position) (break `SplinePoint` (`SplineComponent.GetSplinePointAt` _spline 1 "Local")))
  (`KismetSystemLibrary.PrintString` (`KismetStringLibrary.Conv_IntToString` (`SplineComponent.GetNumberOfSplinePoints` _spline)))
  (`KismetSystemLibrary.PrintString` (`KismetStringLibrary.Conv_VectorToString` _returnvalue_position)))

(event `self.Interact`
  (bind _returnvalue (`GameplayStatics.GetPlayerController` 0))
  (bind _returnvalue_2 (`|CreateWidget` "/Game/Core/Widgets/W_Puzzle2.W_Puzzle2_C" _returnvalue))
  (bind _output_get (set `self.Puzzle Widget` _returnvalue_2))
  (`UserWidget.AddToViewport` _output_get 0)
  (`WidgetBlueprintLibrary.SetInputMode_GameAndUIEx` _returnvalue _returnvalue_2)
  (`CharacterMovementComponent.DisableMovement` (`Character.CharacterMovement` (`GameplayStatics.GetPlayerCharacter` 0))))

(event `self.Start`
  (`parent.Start`))

(event `self.Finish`
  (`parent.Finish`))

(fn `UserConstructionScript`
  (`parent.UserConstructionScript`)
  (`KismetSystemLibrary.PrintString` "constructino scropt"))