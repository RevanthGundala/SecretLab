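; BP_Puzzle1 is an interactable puzzle object that opens the W_Puzzle1 UI when the player interacts with it.
; Interact creates and displays the widget, switches to UI-only input with a visible cursor, and disables the player character's movement.
; Back removes the widget, restores game-only input, hides the cursor, and sets movement back to Walking.
; The puzzle logic itself is not in this Blueprint.
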(event `/Game/Core/Blueprints/BPI_Puzzle.Interact`
  (bind _returnvalue (`GameplayStatics.GetPlayerController` 0))
  (bind _returnvalue_2 (`|CreateWidget` "/Game/Core/Widgets/W_Puzzle1.W_Puzzle1_C" _returnvalue))
  (bind _output_get (set `self.Puzzle Widget` _returnvalue_2))
  (`UserWidget.AddToViewport` _output_get 0)
  (`WidgetBlueprintLibrary.SetInputMode_UIOnlyEx` _returnvalue _output_get "DoNotLock" true)
  (set `PlayerController.bShowMouseCursor` true _returnvalue)
  (`CharacterMovementComponent.DisableMovement` (`Character.CharacterMovement` (`GameplayStatics.GetPlayerCharacter` 0))))

(event `/Game/Core/Blueprints/BPI_Puzzle.Back`
  (bind _returnvalue (`GameplayStatics.GetPlayerController` 0))
  (`Widget.RemoveFromParent` (`self.Puzzle Widget`))
  (`WidgetBlueprintLibrary.SetInputMode_GameOnly` _returnvalue)
  (set `PlayerController.bShowMouseCursor` false _returnvalue)
  (`CharacterMovementComponent.SetMovementMode` (`Character.CharacterMovement` (`GameplayStatics.GetPlayerCharacter` 0)) "MOVE_Walking" 0))

(fn `UserConstructionScript`)