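; BP_Exit is an exit actor that plays a level sequence when the player wins.
; On BeginPlay it creates a level sequence player from its assigned sequence and casts player character 0 to BP_FirstPersonCharacter.
; It binds to that character's OnWin event, and the handler plays the stored sequence.
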(event `self.ReceiveBeginPlay`
  (bind _outactor (`LevelSequencePlayer.CreateLevelSequencePlayer` "/Game/Core/Blueprints/Sequence.Sequence"))
  (set `self.Level Sequence` _outactor)
  (bind _asbp_first_person_character (cast `/Game/FirstPerson/Blueprints/BP_FirstPersonCharacter` (`GameplayStatics.GetPlayerCharacter` 0)))
  (set `self.As BP First Person Character` _asbp_first_person_character)
  (add `/Game/FirstPerson/Blueprints/BP_FirstPersonCharacter.OnWin` (`self.As BP First Person Character`) (delegate `Handle Win`)))

(event `Handle Win`
  (`MovieSceneSequencePlayer.Play` (`LevelSequenceActor.SequencePlayer` (`self.Level Sequence`))))

(fn `UserConstructionScript`)